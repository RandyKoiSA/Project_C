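; Actor component that holds a player or actor inventory as an array of item structs, each with a name, a granted ability class and a Blueprint class.
; AddItemToInventory appends an item to that array.
; PrintInformation is a debug helper that loops over the array and prints each entry's index, name and class display names.
; The event graph has no active logic.
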(event EventBeginPlay)

(event EventTick
  (params (DeltaSeconds :type Float%20%28single-precision%29)))

(fn AddItemtoInventory
  (params (Item :type S%20Item%20Structure))
  (Utilities|Array|Add (.inventory (Variables|Default|GetInventory)) Item))

(fn PrintInformation
  (for (_array_element _array_index) (.inventory (Variables|Default|GetInventory))
    (Development|PrintString (Utilities|String|ToString(Integer) _array_index))
    (Development|PrintString (Utilities|String|ToString(Text) (.name _array_element)))
    (Development|PrintString (Utilities|GetClassDisplayName (.grantedabillity _array_element)))
    (Development|PrintString (Utilities|GetClassDisplayName (.blueprint _array_element)))))