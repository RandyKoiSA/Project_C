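; BP_Player is the player character, with camera-yaw-relative movement, a slower walk while held, melee attacks and death handling.
; BeginPlay attaches a Bow_stick weapon to the hand socket, grants the GA_Melee ability and makes head, arm and leg meshes follow the body's pose.
; MeleeAttack activates that ability through the Ability System, while Die plays a montage, then destroys character and weapon.
; Left and Right keys toggle helmet and chestplate meshes.
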(event Custom|Melee%20Attack
  ;[1 1 1] Melee Event
  (Abilities|TryActivateAbilitybyClass (Variables|Default|GetAbilitySystemComp) "/Game/Project_C/Blueprints/GameplayAbillities/Melee/GA_Melee.GA_Melee_C" true))

(event EventBeginPlay
  (Utilities|FlowControl|Sequence
    (:then_0
      (bind _returnvalue (Game|SpawnActorfromClass "/Game/Project_C/Blueprints/bow_stick.bow_stick_C" (Transformation|GetWorldTransform (Variables|Character|GetMesh)) "Undefined" 0 0))
      (bind _output_get (Variables|Default|SetPrimaryWeapon _returnvalue))
      (Transformation|AttachComponentToComponent _output_get (Variables|Character|GetMesh) "Hand_RSocket" "SnapToTarget" "SnapToTarget" "SnapToTarget" true)
      (Actor|SetOwner (Variables|Default|GetPrimaryWeapon) self))
    (:then_1
      (Class|PlayerCharacter|AcquireAbillity "/Game/Project_C/Blueprints/GameplayAbillities/Melee/GA_Melee.GA_Melee_C"))
    (:then_2
      (Class|SkinnedMeshComponent|SetMasterPoseComponent (Variables|Default|GetHeadMesh) (Variables|Character|GetMesh) false))))

(event EventDie
  ;[1 1 1] Die Event
  (bind _returnvalue (Animation|PlayAnimMontage "/Game/Project_C/CuteCharacter/Animations/montage_dying.montage_dying" 1.0 "None"))
  (Utilities|FlowControl|Delay _returnvalue)
  (CallFunction|OnDeath))

(event Input|ActionEvents|InputActionWalk
  (params (Key :type Key%20Structure :default "None"))
  (bind _charactermovement (Variables|Character|GetCharacterMovement))
  ;[1 1 1] Walk Action
  (:Pressed
    (Variables|/Script/Engine.CharacterMovementComponent|SetMaxWalkSpeed _charactermovement 3e+02))
  (:Released
    (Variables|/Script/Engine.CharacterMovementComponent|SetMaxWalkSpeed _charactermovement 5e+02)))

(event Input|AxisEvents|InputAxisMoveForward
  (params (AxisValue :type Float%20%28single-precision%29))
  ;[1 1 1] Movement
  (Pawn|Input|AddMovementInput (Math|Vector|GetForwardVector (Math|Rotator|MakeRotator 0.0 0.0 (.yaw (Pawn|GetControlRotation :!class /Script/Engine.Pawn)))) AxisValue false))

(event Input|AxisEvents|InputAxisMoveRight
  (params (AxisValue :type Float%20%28single-precision%29))
  ;[1 1 1] Movement
  (Pawn|Input|AddMovementInput (Math|Vector|GetRightVector (Math|Rotator|MakeRotator 0.0 0.0 (.yaw (Pawn|GetControlRotation :!class /Script/Engine.Pawn)))) AxisValue false))

(event Input|KeyboardEvents|Left
  (params (Key :type Key%20Structure :default "None"))
  (bind _headmesh (Variables|Default|GetHeadMesh))
  (:Pressed
    (Utilities|FlowControl|FlipFlop
      (:A
        (Class|SkinnedMeshComponent|SetSkeletalMesh _headmesh "/Game/Project_C/CuteCharacter/ModularParts/Head/leather_helmet.leather_helmet" true))
      (:B
        (Class|SkinnedMeshComponent|SetSkeletalMesh _headmesh "/Game/Project_C/CuteCharacter/ModularParts/Head/cutecharacter_head.cutecharacter_head" true)))))

(event Input|KeyboardEvents|Right
  (params (Key :type Key%20Structure :default "None"))
  (bind _mesh (Variables|Character|GetMesh))
  (:Pressed
    (Utilities|FlowControl|FlipFlop
      (:A
        (Class|SkinnedMeshComponent|SetSkeletalMesh _mesh "/Game/Project_C/CuteCharacter/ModularParts/Body/iron_chestplate.iron_chestplate" true))
      (:B
        (Class|SkinnedMeshComponent|SetSkeletalMesh _mesh "/Game/Project_C/CuteCharacter/ModularParts/Body/cutecharacter_torso.cutecharacter_torso" true)))))

(fn ConstructionScript)

(fn OnDeath
  (Actor|DestroyActor)
  (Actor|DestroyActor (Variables|Default|GetPrimaryWeapon)))