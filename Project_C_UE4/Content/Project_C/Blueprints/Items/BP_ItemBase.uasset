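; Base pickup item actor that carries an ItemInfo struct for the player's inventory.
; The construction script writes the actor's own class into ItemInfo and sets mesh physics from IsPhysicOn.
; When physics is on, BeginPlay launches the mesh with a mostly upward, randomized impulse.
; BeingPickedUp adds ItemInfo to the InventoryComponent on player 0's PC_Player controller, then destroys the actor.
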(event EventBeginPlay
  (if (Variables|Default|GetbIsPhysicOn?)
    (CallFunction|PulseItem)))

(event Collision|EventActorBeginOverlap
  (params (OtherActor :type Actor%20Object%20Reference)))

(event EventTick
  (params (DeltaSeconds :type Float%20%28single-precision%29)))

(event EventBeingPickedUp
  (params (Instigator :type Actor%20Object%20Reference))
  (bind _aspc_player (Utilities|Casting|CastToPC_Player (Game|GetPlayerController 0)))
  (Default|AddItemtoInventory (Variables|/Game/Project_C/Blueprints/Core/PC_Player.PC_Player_C|GetInventoryComponent _aspc_player) (Variables|Default|GetItemInfo))
  (Actor|DestroyActor))

(fn ConstructionScript
  (Variables|Default|SetItemInfo (Utilities|Struct|MakeS_Item (.name (Variables|Default|GetItemInfo)) (.description (Variables|Default|GetItemInfo)) (.icon (Variables|Default|GetItemInfo)) (.quantity (Variables|Default|GetItemInfo)) (.maxquantity (Variables|Default|GetItemInfo)) (.category (Variables|Default|GetItemInfo)) (.grantedabillity (Variables|Default|GetItemInfo)) (.bisconsumable (Variables|Default|GetItemInfo)) (Utilities|GetClass self)))
  (Physics|SetSimulatePhysics (Variables|Default|GetItemMesh) (Variables|Default|GetbIsPhysicOn?)))

(fn PulseItem
  (Physics|AddImpulse (Variables|Default|GetItemMesh) (Math|Vector|MakeVector (Math|Random|RandomFloatinRange 2e+02 8e+02) (Math|Random|RandomFloatinRange 2e+02 8e+02) 3.5e+03) "None" false))