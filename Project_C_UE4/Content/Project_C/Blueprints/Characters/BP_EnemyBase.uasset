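; BP_EnemyBase is a base enemy character Blueprint that uses the Gameplay Ability System and shows a health bar widget.
; When health changes, it casts the HealthBar component's widget to WBP_HealthBar and sets its fill to health over max health.
; A UsePrimaryAbility event activates the ability class in PrimarySlot through the ability system component, with remote activation allowed.
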(event Custom|Use%20Primary%20Ability
  ;[1 1 1] Primary Ability
  (Abilities|TryActivateAbilitybyClass (Variables|Default|GetAbilitySystemComp) (Variables|Default|GetPrimarySlot) true))

(event EventBeginPlay
  (|CallParentFunction) ; This node is disabled and will not be called.\nDrag off pins to build functionality.
)

(event Collision|EventActorBeginOverlap
  (params (OtherActor :type Actor%20Object%20Reference)))

(event EventTick
  (params (DeltaSeconds :type Float%20%28single-precision%29))
  (|CallParentFunction DeltaSeconds) ; This node is disabled and will not be called.\nDrag off pins to build functionality.
)

(event EventOnhealthChanged
  (params (Health :type Float%20%28single-precision%29) (Maxhealth :type Float%20%28single-precision%29))
  ;[1 1 1] OnHealthChange
  (bind _aswbp_health_bar (Utilities|Casting|CastToWBP_HealthBar (UserInterface|GetUserWidgetObject (Variables|Default|GetHealthBar))))
  (Default|SetPercentage _aswbp_health_bar (/ Health Maxhealth)))

(fn ConstructionScript
  (|CallParentFunction))