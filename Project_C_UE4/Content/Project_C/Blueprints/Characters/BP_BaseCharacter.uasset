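; Base character with camera-yaw-relative movement, a walk toggle on hold, modular body meshes and an equipment system.
; Head, arm and leg meshes follow the main mesh via master pose.
; Equip routes items by category: weapons spawn and attach to hand sockets, armor swaps slot meshes and materials, and both pass granted abilities to equip-ability calls.
; Die plays a montage, then OnDeath destroys the character and primary weapon.
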(event EventDie
  ;[1 1 1] Die Event
  (bind _returnvalue (Animation|PlayAnimMontage "/Game/Project_C/CuteCharacter/Animations/montage_dying.montage_dying" 1.0 "None"))
  (Utilities|FlowControl|Delay _returnvalue)
  (CallFunction|OnDeath))

(event Input|ActionEvents|InputActionWalk
  (params (Key :type Key%20Structure :default "None"))
  (bind _charactermovement (Variables|Character|GetCharacterMovement))
  ;[1 1 1] Walk Action
  (:Pressed
    (Variables|/Script/Engine.CharacterMovementComponent|SetMaxWalkSpeed _charactermovement 3e+02))
  (:Released
    (Variables|/Script/Engine.CharacterMovementComponent|SetMaxWalkSpeed _charactermovement 5e+02)))

(event Input|AxisEvents|InputAxisMoveForward
  (params (AxisValue :type Float%20%28single-precision%29))
  ;[1 1 1] Movement
  (Pawn|Input|AddMovementInput (Math|Vector|GetForwardVector (Math|Rotator|MakeRotator 0.0 0.0 (.yaw (Pawn|GetControlRotation :!class /Script/Engine.Pawn)))) AxisValue false))

(event Input|AxisEvents|InputAxisMoveRight
  (params (AxisValue :type Float%20%28single-precision%29))
  ;[1 1 1] Movement
  (Pawn|Input|AddMovementInput (Math|Vector|GetRightVector (Math|Rotator|MakeRotator 0.0 0.0 (.yaw (Pawn|GetControlRotation :!class /Script/Engine.Pawn)))) AxisValue false))

(fn ConstructionScript
  (Class|SkinnedMeshComponent|SetMasterPoseComponent (Variables|Default|GetHeadMesh) (Variables|Character|GetMesh) false))

(fn OnDeath
  (bind _equipment (Variables|Default|GetEquipment))
  (Actor|DestroyActor)
  (Utilities|IsValid (.primaryweaponinstance _equipment)
    (:Is%20Valid
      (Actor|DestroyActor (.primaryweaponinstance _equipment)))
    (:Is%20Not%20Valid
      _))
  (Input|DisableInput (Game|GetPlayerController 0)))

(fn EquipPrimaryWeapon
  (params (Item :type S%20Item%20Structure))
  (bind (_name _description _icon _quantity _maxquantity _category _grantedabillity _bisconsumable _blueprint) (Utilities|Struct|BreakS_Item Item))
  (switch Utilities|FlowControl|Switch|SwitchonE_ItemCategory _category
    (:NewEnumerator5
      (bind _asbp_weapon_base (Utilities|Casting|CastToBP_WeaponBaseClass _blueprint))
      ;[1 1 1] Destroy previous primary weapon
      (Utilities|IsValid (.primaryweaponinstance (Variables|Default|GetEquipment))
        (:Is%20Valid
          (Actor|DestroyActor (.primaryweaponinstance (Variables|Default|GetEquipment))))
        (:Is%20Not%20Valid
          _))
      (bind _returnvalue (Game|SpawnActorfromClass _asbp_weapon_base (Transformation|GetWorldTransform (Variables|Character|GetMesh)) "Undefined" 0 0))
      (bind _output_get (LocalVariables|SetPrimaryWeapon _returnvalue))
      (Variables|/Game/Project_C/Blueprints/Items/BP_ItemBase.BP_ItemBase_C|SetbIsPickedUp _output_get true)
      (Variables|Default|SetEquipment (Utilities|Struct|MakeS_PlayerEquipment _output_get (.secondaryweaponinstance (Variables|Default|GetEquipment)) (.headclass (Variables|Default|GetEquipment)) (.chestclass (Variables|Default|GetEquipment)) (.armsclass (Variables|Default|GetEquipment)) (.legsclass (Variables|Default|GetEquipment))))
      (Transformation|AttachComponentToComponent _output_get (Variables|Character|GetMesh) "Hand_RSocket" "SnapToTarget" "SnapToTarget" "SnapToTarget" true)
      (Actor|SetOwner (LocalVariables|GetPrimaryWeapon) self)
      (Class|PlayerCharacter|EquipPrimaryAbility (.grantedabillity (Variables|/Game/Project_C/Blueprints/Items/BP_ItemBase.BP_ItemBase_C|GetItemInfo (LocalVariables|GetPrimaryWeapon)))))
    (:NewEnumerator6
      (CallFunction|EquipSecondaryWeapon Item))
    (:NewEnumerator11
      (CallFunction|EquipArmor Item))))

(fn EquipSecondaryWeapon
  (params (Item :type S%20Item%20Structure))
  (bind (_name _description _icon _quantity _maxquantity _category _grantedabillity _bisconsumable _blueprint) (Utilities|Struct|BreakS_Item Item))
  (switch Utilities|FlowControl|Switch|SwitchonE_ItemCategory _category
    (:NewEnumerator5
      (CallFunction|EquipPrimaryWeapon Item))
    (:NewEnumerator6
      (bind _asbp_weapon_base (Utilities|Casting|CastToBP_WeaponBaseClass _blueprint))
      ;[1 1 1] Destroy previous secondary weapon
      (Utilities|IsValid (.secondaryweaponinstance (Variables|Default|GetEquipment))
        (:Is%20Valid
          (Actor|DestroyActor (.secondaryweaponinstance (Variables|Default|GetEquipment))))
        (:Is%20Not%20Valid
          _))
      (bind _returnvalue (Game|SpawnActorfromClass _asbp_weapon_base (Transformation|GetWorldTransform (Variables|Character|GetMesh)) "Undefined" 0 0))
      (bind _output_get (LocalVariables|SetSecondaryWeapon _returnvalue))
      (Variables|/Game/Project_C/Blueprints/Items/BP_ItemBase.BP_ItemBase_C|SetbIsPickedUp _output_get true)
      (Variables|Default|SetEquipment (Utilities|Struct|MakeS_PlayerEquipment (.primaryweaponinstance (Variables|Default|GetEquipment)) _output_get (.headclass (Variables|Default|GetEquipment)) (.chestclass (Variables|Default|GetEquipment)) (.armsclass (Variables|Default|GetEquipment)) (.legsclass (Variables|Default|GetEquipment))))
      (switch Utilities|FlowControl|Switch|SwitchonE_SecondaryWeaponType (Variables|/Game/Project_C/Blueprints/Items/BP_WeaponBase.BP_WeaponBase_C|GetSecondaryType _output_get)
        (:NewEnumerator0
          (Transformation|AttachComponentToComponent (LocalVariables|GetSecondaryWeapon) (Variables|Character|GetMesh) "Hand_LShield" "SnapToTarget" "SnapToTarget" "SnapToTarget" true))
        (:NewEnumerator1
          (Transformation|AttachComponentToComponent (LocalVariables|GetSecondaryWeapon) (Variables|Character|GetMesh) "Hand_LWeapon" "SnapToTarget" "SnapToTarget" "SnapToTarget" true :!label _label))
        (:NewEnumerator2
          (goto _label)))
      (Actor|SetOwner (LocalVariables|GetSecondaryWeapon) self)
      (if (Utilities|IsValidClass (.grantedabillity (Variables|/Game/Project_C/Blueprints/Items/BP_ItemBase.BP_ItemBase_C|GetItemInfo (LocalVariables|GetSecondaryWeapon))))
        (Class|PlayerCharacter|EquipSecondaryAbility (.grantedabillity (Variables|/Game/Project_C/Blueprints/Items/BP_ItemBase.BP_ItemBase_C|GetItemInfo (LocalVariables|GetSecondaryWeapon))))))
    (:NewEnumerator11
      (CallFunction|EquipArmor Item))))

(fn EquipArmor
  (params (Item :type S%20Item%20Structure))
  (bind (_name _description _icon _quantity _maxquantity _category _grantedabillity _bisconsumable _blueprint) (Utilities|Struct|BreakS_Item Item))
  (bind _legmesh (Variables|Default|GetLegMesh))
  (bind _mesh (Variables|Character|GetMesh))
  (bind _headmesh (Variables|Default|GetHeadMesh))
  (bind _armmesh (Variables|Default|GetArmMesh))
  (LocalVariables|SetGrantedAbillity _grantedabillity)
  (switch Utilities|FlowControl|Switch|SwitchonE_ItemCategory _category
    (:NewEnumerator5
      (CallFunction|EquipPrimaryWeapon Item))
    (:NewEnumerator6
      (CallFunction|EquipSecondaryWeapon Item))
    (:NewEnumerator11
      (bind _asbp_armor_base (Utilities|Casting|CastToBP_ArmorBaseClass _blueprint))
      (bind _output_get (LocalVariables|SetArmorBase _asbp_armor_base))
      (switch Utilities|FlowControl|Switch|SwitchonE_ArmorType (.ArmorType (Utilities|GetClassDefaults _output_get))
        (:NewEnumerator0
          ;[1 1 1] Head Equip
          (Class|SkinnedMeshComponent|SetSkeletalMesh _headmesh (.SkeletalMesh (Utilities|GetClassDefaults (LocalVariables|GetArmorBase))) true)
          (Rendering|Material|SetMaterial _headmesh 0 (.Material_01 (Utilities|GetClassDefaults (LocalVariables|GetArmorBase))))
          (Rendering|Material|SetMaterial _headmesh 1 (.Material_02 (Utilities|GetClassDefaults (LocalVariables|GetArmorBase))))
          (Variables|Default|SetEquipment (Utilities|Struct|MakeS_PlayerEquipment (.primaryweaponinstance (Variables|Default|GetEquipment)) (.secondaryweaponinstance (Variables|Default|GetEquipment)) (LocalVariables|GetArmorBase) (.chestclass (Variables|Default|GetEquipment)) (.armsclass (Variables|Default|GetEquipment)) (.legsclass (Variables|Default|GetEquipment))))
          (Class|PlayerCharacter|EquipHeadSlot (LocalVariables|GetGrantedAbillity)))
        (:NewEnumerator1
          ;[1 1 1] Chest Equip
          (Class|SkinnedMeshComponent|SetSkeletalMesh _mesh (.SkeletalMesh (Utilities|GetClassDefaults (LocalVariables|GetArmorBase))) true)
          (Rendering|Material|SetMaterial _mesh 0 (.Material_01 (Utilities|GetClassDefaults (LocalVariables|GetArmorBase))))
          (Rendering|Material|SetMaterial _mesh 1 (.Material_02 (Utilities|GetClassDefaults (LocalVariables|GetArmorBase))))
          (Variables|Default|SetEquipment (Utilities|Struct|MakeS_PlayerEquipment (.primaryweaponinstance (Variables|Default|GetEquipment)) (.secondaryweaponinstance (Variables|Default|GetEquipment)) (.headclass (Variables|Default|GetEquipment)) (LocalVariables|GetArmorBase) (.armsclass (Variables|Default|GetEquipment)) (.legsclass (Variables|Default|GetEquipment))))
          (Class|PlayerCharacter|EquipChestSlot (LocalVariables|GetGrantedAbillity)))
        (:NewEnumerator2
          ;[1 1 1] Arms Equip
          (Class|SkinnedMeshComponent|SetSkeletalMesh _armmesh (.SkeletalMesh (Utilities|GetClassDefaults (LocalVariables|GetArmorBase))) true)
          (Rendering|Material|SetMaterial _armmesh 0 (.Material_01 (Utilities|GetClassDefaults (LocalVariables|GetArmorBase))))
          (Rendering|Material|SetMaterial _armmesh 1 (.Material_02 (Utilities|GetClassDefaults (LocalVariables|GetArmorBase))))
          (Variables|Default|SetEquipment (Utilities|Struct|MakeS_PlayerEquipment (.primaryweaponinstance (Variables|Default|GetEquipment)) (.secondaryweaponinstance (Variables|Default|GetEquipment)) (.headclass (Variables|Default|GetEquipment)) (.chestclass (Variables|Default|GetEquipment)) (LocalVariables|GetArmorBase) (.legsclass (Variables|Default|GetEquipment))))
          (Class|PlayerCharacter|EquipArmsSlot (LocalVariables|GetGrantedAbillity)))
        (:NewEnumerator3
          ;[1 1 1] Leg Equip
          (Class|SkinnedMeshComponent|SetSkeletalMesh _legmesh (.SkeletalMesh (Utilities|GetClassDefaults (LocalVariables|GetArmorBase))) true)
          (Rendering|Material|SetMaterial _legmesh 0 (.Material_01 (Utilities|GetClassDefaults (LocalVariables|GetArmorBase))))
          (Rendering|Material|SetMaterial _legmesh 1 (.Material_02 (Utilities|GetClassDefaults (LocalVariables|GetArmorBase))))
          (Variables|Default|SetEquipment (Utilities|Struct|MakeS_PlayerEquipment (.primaryweaponinstance (Variables|Default|GetEquipment)) (.secondaryweaponinstance (Variables|Default|GetEquipment)) (.headclass (Variables|Default|GetEquipment)) (.chestclass (Variables|Default|GetEquipment)) (.armsclass (Variables|Default|GetEquipment)) (LocalVariables|GetArmorBase)))
          (Class|PlayerCharacter|EquipLegsSlot (LocalVariables|GetGrantedAbillity)))))))

(fn Equip
  (params (Item :type S%20Item%20Structure))
  (switch Utilities|FlowControl|Switch|SwitchonE_ItemCategory (.Category (Utilities|Struct|BreakS_Item Item))
    (:NewEnumerator5
      (CallFunction|EquipPrimaryWeapon Item))
    (:NewEnumerator6
      (CallFunction|EquipSecondaryWeapon Item))
    (:NewEnumerator11
      (CallFunction|EquipArmor Item))))