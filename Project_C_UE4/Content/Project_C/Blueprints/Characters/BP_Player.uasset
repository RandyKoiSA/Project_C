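; Player character Blueprint that connects Gameplay Ability System ability slots and health/mana changes to gameplay and the HUD.
; Health and mana change events cast through HUD_Project_C to WBP_PrimaryUI and set each glass ball to the current-to-max ratio.
; Primary, secondary and four skill events activate their slot's ability class on the AbilitySystemComp, with remote activation allowed.
; Only primary and secondary print success or failure; BeginPlay and construction just call the parent.
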(event Custom|Use%20Primary%20Ability
  ;[1 1 1] Primary Ability
  (bind _returnvalue (Abilities|TryActivateAbilitybyClass (Variables|Default|GetAbilitySystemComp) (Variables|Default|GetPrimarySlot) true))
  (if _returnvalue
    (Development|PrintString "BP_Player: Successfully Cast Primary Ability" true true "(R=0.000000,G=1.000000,B=0.031514,A=1.000000)")
    (else
      (Development|PrintString "BP_Player: Failed To Cast Primary Ability" true true "(R=1.000000,G=0.000000,B=0.093043,A=1.000000)"))))

(event Custom|Use%20Secondary%20Ability
  ;[1 1 1] Secondary Abillity
  (bind _returnvalue (Abilities|TryActivateAbilitybyClass (Variables|Default|GetAbilitySystemComp) (Variables|Default|GetSecondarySlot) true))
  (if _returnvalue
    (Development|PrintString "BP_Player: Successfully Cast Secondary Ability" true true "(R=0.000000,G=1.000000,B=0.031514,A=1.000000)")
    (else
      (Development|PrintString "BP_Player: Failed To Cast Secondary Ability" true true "(R=1.000000,G=0.000000,B=0.093043,A=1.000000)"))))

(event Custom|Use%20Skill%20One
  ;[1 1 1] Skill One Ability
  (Abilities|TryActivateAbilitybyClass (Variables|Default|GetAbilitySystemComp) (Variables|Default|GetSkillOneSlot) true))

(event Custom|Use%20Skill%20Two
  ;[1 1 1] Skill Two Ability
  (Abilities|TryActivateAbilitybyClass (Variables|Default|GetAbilitySystemComp) (Variables|Default|GetSkillTwoSlot) true))

(event Custom|Use%20Skill%20Three
  ;[1 1 1] Skill Three Ability
  (Abilities|TryActivateAbilitybyClass (Variables|Default|GetAbilitySystemComp) (Variables|Default|GetSkillThreeSlot) true))

(event Custom|Use%20Skill%20Four
  ;[1 1 1] Skill Four Ability
  (Abilities|TryActivateAbilitybyClass (Variables|Default|GetAbilitySystemComp) (Variables|Default|GetSkillFourSlot) true))

(event EventBeginPlay
  (|CallParentFunction))

(event Collision|EventActorBeginOverlap
  (params (OtherActor :type Actor%20Object%20Reference)))

(event EventTick
  (params (DeltaSeconds :type Float%20%28single-precision%29)))

(event EventOnhealthChanged
  (params (Health :type Float%20%28single-precision%29) (Maxhealth :type Float%20%28single-precision%29))
  ;[1 1 1] On Health Changed
  (bind _ashud_project_c (Utilities|Casting|CastToHUD_Project_C (HUD|GetHUD (Game|GetPlayerController 0))))
  (bind _aswbp_primary_ui (Utilities|Casting|CastToWBP_PrimaryUI (Variables|/Game/Project_C/Blueprints/Core/HUD_Project_C.HUD_Project_C_C|GetPrimaryUI _ashud_project_c)))
  (Default|SetPercentage (Variables|/Game/Project_C/Blueprints/Widgets/WBP_PrimaryUI.WBP_PrimaryUI_C|GetHealth_GlassBall _aswbp_primary_ui) (/ Health Maxhealth)))

(event EventOnManaChanged
  (params (Mana :type Float%20%28single-precision%29) (MaxMana :type Float%20%28single-precision%29))
  ;[1 1 1] On Mana Changed
  (bind _ashud_project_c (Utilities|Casting|CastToHUD_Project_C (HUD|GetHUD (Game|GetPlayerController 0))))
  (bind _aswbp_primary_ui (Utilities|Casting|CastToWBP_PrimaryUI (Variables|/Game/Project_C/Blueprints/Core/HUD_Project_C.HUD_Project_C_C|GetPrimaryUI _ashud_project_c)))
  (Default|SetPercentage (Variables|/Game/Project_C/Blueprints/Widgets/WBP_PrimaryUI.WBP_PrimaryUI_C|GetMana_GlassBall _aswbp_primary_ui) (/ Mana MaxMana)))

(fn ConstructionScript
  (|CallParentFunction))